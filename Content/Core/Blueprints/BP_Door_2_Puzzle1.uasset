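; BP_Door_2_Puzzle1 is a door actor, named for the first puzzle, that slides open when its Open event fires.
; Open caches the current location, then a timeline lerps the actor a fixed distance along negative world X.
; A flag blocks retriggering while the slide runs and clears on finish, so a later call moves the door again from its new position.
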(event Custom|Open
  (if (not (Variables|Default|GetisDoorOpening))
    (Variables|Default|SetisDoorOpening true)
    (Variables|Default|SetDoorLocation (Transformation|GetActorLocation))
    (bind _openspeed (Timeline|OpenDoorAnim PlayFromStart)
      (:Update
        (Transformation|SetActorLocation (Math|Vector|Lerp(Vector) (Variables|Default|GetDoorLocation) (Math|Vector|MakeVector (+ (.X (Math|Vector|BreakVector (Variables|Default|GetDoorLocation))) -3e+02) (.Y (Math|Vector|BreakVector (Variables|Default|GetDoorLocation))) (.Z (Math|Vector|BreakVector (Variables|Default|GetDoorLocation)))) _openspeed) false false))
      (:Finished
        (Variables|Default|SetisDoorOpening false)))))

(fn ConstructionScript)