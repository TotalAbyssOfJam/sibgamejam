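; BP_FinalExit is an interactable exit device that plays an electrified launch effect when the player activates it with E.
; A box overlap enables input; E spawns BP_ActorDeath at the character mesh's transform, hides that mesh and disables input.
; Activation also applies a dynamic glow material to the sphere and starts shield particles, Niagara and electric audio.
; Once launched, Tick slowly rotates the ring and randomly flickers the point light.
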(event OnComponentBeginOverlap(Box)
  (params (OverlappedComponent :type Primitive%20Component%20Object%20Reference) (OtherActor :type Actor%20Object%20Reference) (OtherComp :type Primitive%20Component%20Object%20Reference) (OtherBodyIndex :type Integer) (bFromSweep :type Boolean) (SweepResult :type Hit%20Result%20Structure%20%28by%20ref%29))
  (Input|EnableInput (Game|GetPlayerController 0)))

(event EventTick
  (params (DeltaSeconds :type Float%20%28single-precision%29))
  (if (Variables|Default|GetIsLaunch)
    (Transformation|AddWorldRotation (Variables|Default|GetRing) "0, 0,0.050000" false false)
    (Rendering|Components|Light|SetIntensity (Variables|Default|GetPointLight) (* (Math|Random|RandomFloat) 1.5e+04))))

(event Input|KeyboardEvents|E
  (params (Key :type Key%20Structure :default "None"))
  (bind _returnvalue (Game|GetPlayerController 0))
  (:Pressed
    (bind _asbp_character (Utilities|Casting|CastToBP_Character (Game|Player|GetPlayerPawn 0)))
    (Game|SpawnActorfromClass "/Game/Core/Blueprints/BP_ActorDeath.BP_ActorDeath_C" (Transformation|GetWorldTransform (Variables|/Script/Engine.Character|GetMesh _asbp_character)) "Undefined" 0 0)
    (Rendering|SetVisibility (Variables|/Script/Engine.Character|GetMesh _asbp_character) false false)
    (Variables|Default|SetIsLaunch true)
    (bind _returnvalue_2 (Rendering|Material|CreateDynamicMaterialInstance "/Game/Core/VFX/M_Scifi_Glow_Inst.M_Scifi_Glow_Inst" "Super" :!class /Script/Engine.KismetMaterialLibrary))
    (Variables|Default|SetMaterial _returnvalue_2)
    (Rendering|Material|SetMaterial (Variables|Default|GetSphere) 0 (Variables|Default|GetMaterial))
    (Components|Activation|SetActive (Variables|Default|GetPS_ElectroShield) true false)
    (Components|Activation|SetActive (Variables|Default|GetNiagara) true false)
    (Audio|SpawnSoundatLocation "/Game/Core/VFX/electric_Cue.electric_Cue" (Transformation|GetActorLocation) "0, 0, 0" 1.0 1.0 0.0 0 0)
    (Input|DisableInput (Game|GetPlayerController 0))
    (Input|DisableInput _returnvalue _returnvalue)
    (bind _ascharacter (Utilities|Casting|CastToCharacter (Game|Player|GetPlayerPawn 0)))
    (Physics|SetSimulatePhysics (Variables|/Script/Engine.Character|GetMesh _ascharacter) false)))

(fn ConstructionScript)